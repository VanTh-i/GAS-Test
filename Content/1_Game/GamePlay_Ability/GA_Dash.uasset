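; GA_Dash is a Gameplay Ability that dashes the avatar along its forward vector.
; After committing, it applies a short constant root motion force that keeps its last velocity on finish, and plays the dash montage alongside it.
; When the force finishes it stops the montage, and any montage exit ends the ability, as does a failed commit.
; Ending prints a debug string.
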(event Ability|EventActivateAbility
  (bind _returnvalue (Ability|CommitAbility))
  (if _returnvalue
    (Ability|Tasks|ApplyRootMotionConstantForce "None" (Transformation|GetActorForwardVector (Ability|GetAvatarActorfromActorInfo)) 1e+03 0.3 false 0 "MaintainLastRootMotionVelocity"
      (:then
        (|PlayMontageandWaitProxy "None" (Variables|Default|GetDashAnim) 1.0 "None" true 1.0 0.0 false
          (:OnCompleted
            _)
          (:OnBlendOut
            _)
          (:OnInterrupted
            _)
          (:OnCancelled
            _))
        (Ability|EndAbility))
      (:OnFinish
        (Animation|Montage|MontageStop -1.0)))
    (else
      (Ability|EndAbility))))

(event Ability|EventOnEndAbility
  (params (bWasCancelled :type Boolean))
  (Development|PrintString "End"))